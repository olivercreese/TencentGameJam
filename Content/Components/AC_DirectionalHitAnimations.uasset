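; Actor component that plays front, rear, left or right hit-reaction montages on a skeletal mesh based on a hit direction angle.
; PlayHitAnim sorts the signed angle into a frontal cone, two side sectors and a rear sector, then calls the matching event.
; Each event sets IsAnimPlaying while its montage plays and clears it on blend out or interruption.
; Only the left montage is set not to stop other montages.
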(event `PlayRightHitAnim`
  (params (InSkeletalMeshComponent :type "SkeletalMeshComponent Object Reference"))
  (`|PlayMontage` InSkeletalMeshComponent (`self.RightHitAnimation`)
    (:`then`
      (set `self.IsAnimPlaying` true))
    (:`OnBlendOut`
      (set `self.IsAnimPlaying` false :!label _label))
    (:`OnInterrupted`
      (goto _label))))

(event `PlayRearHitAnim`
  (params (InSkeletalMeshComponent :type "SkeletalMeshComponent Object Reference"))
  (`|PlayMontage` InSkeletalMeshComponent (`self.RearHitAnimation`)
    (:`then`
      (set `self.IsAnimPlaying` true))
    (:`OnBlendOut`
      (set `self.IsAnimPlaying` false :!label _label_2))
    (:`OnInterrupted`
      (goto _label_2))))

(event `PlayFrontHitAnim`
  (params (InSkeletalMeshComponent :type "SkeletalMeshComponent Object Reference"))
  (`|PlayMontage` InSkeletalMeshComponent (`self.FrontHitAnimation`)
    (:`then`
      (set `self.IsAnimPlaying` true))
    (:`OnBlendOut`
      (set `self.IsAnimPlaying` false :!label _label_3))
    (:`OnInterrupted`
      (goto _label_3))))

(event `PlayLeftHitAnim`
  (params (InSkeletalMeshComponent :type "SkeletalMeshComponent Object Reference"))
  (`|PlayMontage` InSkeletalMeshComponent (`self.LeftHitAnimation`) 1.0 0.0 "None" false
    (:`then`
      (set `self.IsAnimPlaying` true))
    (:`OnBlendOut`
      (set `self.IsAnimPlaying` false :!label _label_4))
    (:`OnInterrupted`
      (goto _label_4))))

(fn `PlayHitAnim`
  (params (Direction :type "Float (double-precision)") (Mesh :type "SkeletalMeshComponent Object Reference"))
  (if (> Direction 0.0)
    (if (and (> Direction 65.0) (< Direction 120.0))
      (`self.PlayRightHitAnim` (`local.Mesh`))
      (elif (< Direction 65.0)
        (`self.PlayFrontHitAnim` (`local.Mesh`))
        (elif (>= Direction 120.0)
          (`self.PlayRearHitAnim` (`local.Mesh`)))))
    (elif (and (< Direction -65.0) (> Direction -120.0))
      (`self.PlayLeftHitAnim` (`local.Mesh`))
      (elif (> Direction -65.0)
        (`self.PlayFrontHitAnim` (`local.Mesh`))
        (elif (<= Direction -120.0)
          (`self.PlayRearHitAnim` (`local.Mesh`)))))))
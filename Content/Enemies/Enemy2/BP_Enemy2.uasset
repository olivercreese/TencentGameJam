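; BP_Enemy2 is a ranged enemy character that attacks by throwing magic projectiles.
; Attack plays a one-handed magic montage and signals attack end on completion or interruption, while the separate Throw event spawns BP_Projectile1 just above the actor's location along its facing.
; SetMovementSpeed maps idle, walking and running states to walk speed, and GetIdealRange returns independently randomized attack and strafe radii within a mid-range band.
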(event `/Game/Enemies/BPI_Enemy.Attack`
  (`|PlayMontage` (`self.Mesh`) "/Game/Assets/Mutant/Anim/Standing_1H_Magic_Attack_02_Montage.Standing_1H_Magic_Attack_02_Montage"
    (:`OnCompleted`
      _)
    (:`OnInterrupted`
      _))
  (`self.OnAttackEnd`))

(event `/Game/Enemies/BPI_Enemy.Throw`
  (bind (_returnvalue_x _returnvalue_y _returnvalue_z) (`KismetMathLibrary.BreakVector` (`self.K2_GetActorLocation`)))
  (`|SpawnActorFromClass` "/Game/Enemies/Enemy2/BP_Projectile1.BP_Projectile1_C" (`KismetMathLibrary.MakeTransform` (`KismetMathLibrary.MakeVector` _returnvalue_x _returnvalue_y (+ _returnvalue_z 10.0)) (`KismetMathLibrary.MakeRotator` (.roll (`KismetMathLibrary.MakeRotFromX` (`KismetMathLibrary.GetForwardVector` (`self.K2_GetActorRotation`)))) 0.0 (.yaw (`KismetMathLibrary.MakeRotFromX` (`KismetMathLibrary.GetForwardVector` (`self.K2_GetActorRotation`)))))) "Undefined" "MultiplyWithRoot" null null))

(fn `GetIdealRange`
  (returns (AttackRadius :type "Float (double-precision)") (StrafeRadius :type "Float (double-precision)"))
  (bind _returnvalue (`KismetMathLibrary.RandomFloatInRange` 600.0 750.0))
  (return _returnvalue _returnvalue))

(fn `SetMovementSpeed`
  (params (MovementState :type "/Game/Enemies/AI/E_MovementSpeed Enum" :default "NewEnumerator0"))
  (returns (Speed :type "Float (double-precision)"))
  (bind _output_get (set `CharacterMovementComponent.MaxWalkSpeed` (select `/Game/Enemies/AI/E_MovementSpeed` MovementState :`NewEnumerator1` 200.0 :`NewEnumerator2` 400.0 :!type "Float (single-precision)") (`self.CharacterMovement`)))
  (return _output_get))

(fn `UserConstructionScript`
  (`parent.UserConstructionScript`))
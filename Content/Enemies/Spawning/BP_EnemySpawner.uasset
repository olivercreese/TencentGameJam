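; Enemy spawner actor that holds a queue of enemy classes and spawns them at its own transform.
; AddEnemyToQueue appends a class and spawns immediately if no BP_Enemy1 overlaps its Sphere.
; A looping timer started on BeginPlay also spawns from the queue front, without that overlap check.
; Each spawn binds to the enemy's death event, and OnEnemyKilled reports defeats to BP_CombatGameMode.
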(event `self.ReceiveBeginPlay`
  (`KismetSystemLibrary.K2_SetTimerDelegate` (delegate `tryToSpawn`) 2.0 true))

(event `tryToSpawn`
  (`self.SpawnEnemy`))

(event `OnEnemyKilled`
  (bind _asbp_combat_game_mode (cast `/Game/Player/BP_CombatGameMode` (`GameplayStatics.GetGameMode`)))
  (`/Game/Player/BP_CombatGameMode.OnEnemyDefeated` _asbp_combat_game_mode))

(fn `AddEnemyToQueue`
  (params (EnemyClass :type "/Game/Enemies/Enemy1/BP_Enemy1 Class Reference (by ref)"))
  (`KismetArrayLibrary.Array_Add` (`self.EnemyQueue`) EnemyClass)
  (if (not (`KismetArrayLibrary.Array_IsValidIndex` (`PrimitiveComponent.GetOverlappingActors` (`self.Sphere`) "/Game/Enemies/Enemy1/BP_Enemy1.BP_Enemy1_C")))
    (`self.SpawnEnemy`)))

(fn `SpawnEnemy`
  (returns (Success :type Boolean))
  (if (`KismetArrayLibrary.Array_IsValidIndex` (`self.EnemyQueue`))
    (bind _returnvalue (`|SpawnActorFromClass` (`|GetArrayItem` (`self.EnemyQueue`)) (`self.GetTransform`) "Undefined" "MultiplyWithRoot" null null))
    (add `/Game/Enemies/Enemy1/BP_Enemy1.OnDeath` _returnvalue (`|CreateDelegate` :!event `OnEnemyKilled`))
    (`KismetArrayLibrary.Array_Remove` (`self.EnemyQueue`))
    (return true)
    (else
      (return false))))

(fn `UserConstructionScript`)
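; BP_Enemy1 is a melee stickman enemy character that alternates two attack montages and signals when each attack ends.
; Hits play directional reactions, knock it back, briefly block further damage, return any held attack token to the player and notify the AI.
; Lethal damage plays a death montage, disables movement and switches the AIC_Enemy state.
; It also exposes token, ideal attack/strafe range and movement speed functions for the AI.
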(event `/Game/Player/BPI_Damage.TakeDamage`
  (params (Damage :type "Float (double-precision)") (DamageDirection :type "Float (double-precision)") (DamageCauser :type "Actor Object Reference"))
  (bind _returnvalue (- (`self.Health`) Damage))
  (if (and (`self.CanBeDamaged`) (not (`self.IsDead?`)))
    (if (> _returnvalue 0.0)
      (set `self.Health` _returnvalue)
      (`/Game/Components/AC_DirectionalHitAnimations.PlayHitAnim` (`self.AC_DirectionalHitAnimations`) DamageDirection (`self.Mesh`))
      (if (`self.HasToken?`)
        (message `/Game/Player/BPI_PLayer.ReturnAttackToken` (`GameplayStatics.GetPlayerCharacter` 0) 1)
        (set `self.HasToken?` false))
      (`self.Knockback` DamageCauser 2000.0)
      (`self.OnTakeDamageSetStateAI`)
      (set `self.CanBeDamaged` false)
      (`KismetSystemLibrary.K2_SetTimerDelegate` (delegate `MakeDamageable`) 0.2)
      (else
        (set `self.IsDead?` true)
        (`CharacterMovementComponent.DisableMovement` (`self.CharacterMovement`))
        (`|PlayMontage` (`self.Mesh`) "/Game/Assets/ROG_Creatures/Stickman/Animations/AM_Stickman_Death.AM_Stickman_Death"
          (:`then`
            (bind _asaic_enemy (cast `/Game/Enemies/AI/AIC_Enemy` (`AIBlueprintHelperLibrary.GetAIController` self)))
            (`/Game/Enemies/AI/AIC_Enemy.SetStateAI` _asaic_enemy "NewEnumerator3" null)))))))

(event `MakeDamageable`
  (set `self.CanBeDamaged` true))

(event `/Game/Enemies/BPI_Enemy.SetHasToken`
  (params (TokenIn :type Boolean))
  (set `self.HasToken?` TokenIn))

(event `/Game/Enemies/BPI_Enemy.Attack`
  (bind _mesh (`self.Mesh`))
  (`/Engine/EditorBlueprintResources/StandardMacros.FlipFlop`
    (:`A`
      (`|PlayMontage` _mesh "/Game/Assets/ROG_Creatures/Stickman/Animations/AM_Stickman_Attack_01.AM_Stickman_Attack_01"
        (:`OnCompleted`
          _)))
    (:`B`
      (`|PlayMontage` _mesh "/Game/Assets/ROG_Creatures/Stickman/Animations/AM_Stickman_Attack_02.AM_Stickman_Attack_02"
        (:`OnCompleted`
          _))))
  (`self.OnAttackEnd`))

(event `Knockback`
  (params (`Other Actor` :type "Actor Object Reference") (`Knockback Amount` :type "Float (double-precision)"))
  (`self.LaunchCharacter` (* (`KismetMathLibrary.Normal` (`KismetMathLibrary.MakeVector` (.x (- (`self.K2_GetActorLocation`) (`self.K2_GetActorLocation` `Other Actor`))) (.y (- (`self.K2_GetActorLocation`) (`self.K2_GetActorLocation` `Other Actor`))))) `Knockback Amount`) true))

(fn `CheckHasToken`
  (returns (TokenOut :type Boolean))
  (return (`self.HasToken?`)))

(fn `GetIdealRange`
  (returns (AttackRadius :type "Float (double-precision)") (StrafeRadius :type "Float (double-precision)"))
  (return 100.0 (`KismetMathLibrary.RandomFloatInRange` 450.0 600.0)))

(fn `SetMovementSpeed`
  (params (MovementState :type "/Game/Enemies/AI/E_MovementSpeed Enum" :default "NewEnumerator0"))
  (returns (Speed :type "Float (double-precision)"))
  (bind _output_get (set `CharacterMovementComponent.MaxWalkSpeed` (select `/Game/Enemies/AI/E_MovementSpeed` MovementState :`NewEnumerator1` 200.0 :`NewEnumerator2` 600.0) (`self.CharacterMovement`)))
  (return _output_get))

(fn `UserConstructionScript`)
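; Combat game mode that runs endless enemy waves through the level's BP_EnemySpawner actors, starting at BeginPlay.
; Each wave's class-to-count pool comes from a data table row keyed by wave number, with randomized counts as fallback.
; Random pool picks are queued on random spawners up to EnemyMaxCount, with defeats triggering refills while enough enemies remain.
; When none remain, it fires the end-wave dispatcher and starts the next wave on a timer.
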(event `self.ReceiveBeginPlay`
  (`self.GetSpawners`)
  (`self.NewWave`))

(fn `BuildEnemyPool`
  (bind _returnvalue (`|GetDataTableRow` "/Game/Enemies/Spawning/WavePoolData.WavePoolData" (`KismetStringLibrary.Conv_StringToName` (`KismetStringLibrary.Conv_IntToString` (`self.WaveNumber`))))
    (:`then`
      (set `self.EnemyPool` (`.EnemyPool_4_5130C8CA435C13C37D46528B7E26D10A` (break `/Game/Enemies/Spawning/FWaveStruct` _returnvalue)))
      (set `self.EnemyRemaining` (`self.GetPoolSize`)))
    (:`RowNotFound`
      (`BlueprintMapLibrary.Map_Add` (`self.EnemyPool`) "/Game/Enemies/Enemy1/BP_Enemy1.BP_Enemy1_C" (`KismetMathLibrary.RandomIntegerInRange` 10 (* (`self.WaveNumber`) 5)))
      (`BlueprintMapLibrary.Map_Add` (`self.EnemyPool`) "/Game/Enemies/Enemy2/BP_Enemy2.BP_Enemy2_C" (`KismetMathLibrary.RandomIntegerInRange` 10 (* (`self.WaveNumber`) 10)))
      (set `self.EnemyRemaining` (`self.GetPoolSize`)))))

(fn `EndWave`
  (`self.OnEndWave`))

(fn `EnterTransition`
  (params (`Transition Period` :type "Float (single-precision)"))
  (bind _returnvalue (`KismetSystemLibrary.K2_SetTimer` null "NewWave" `Transition Period`))
  (set `self.TransitionTimer` _returnvalue)
  (`self.EndWave`))

(fn `GetEnemyFromPool`
  (returns (enem :type "/Game/Enemies/Enemy1/BP_Enemy1 Class Reference"))
  (locals (LocalClassType :type "/Game/Enemies/Enemy1/BP_Enemy1 Class Reference"))
  (bind _keys (`BlueprintMapLibrary.Map_Keys` (`self.EnemyPool`)))
  (bind _output_get (set `local.LocalClassType` (`KismetArrayLibrary.Array_Random` _keys)))
  (bind _returnvalue (- (`BlueprintMapLibrary.Map_Find` (`self.EnemyPool`) _output_get) 1))
  (if (> _returnvalue 0)
    (`BlueprintMapLibrary.Map_Add` (`self.EnemyPool`) (`local.LocalClassType`) _returnvalue)
    (return (`local.LocalClassType`))
    (else
      (`BlueprintMapLibrary.Map_Remove` (`self.EnemyPool`) (`local.LocalClassType`))
      (return (`local.LocalClassType`)))))

(fn `GetPoolSize`
  (returns (PoolSize :type Integer))
  (locals (localSum :type Integer))
  (bind _values (`BlueprintMapLibrary.Map_Values` (`self.EnemyPool`)))
  (for _array_element _values
    (set `local.localSum` (+ (`local.localSum`) _array_element)))
  (return (`local.localSum`)))

(fn `GetSpawners`
  (bind _outactors (`GameplayStatics.GetAllActorsOfClass` "/Game/Enemies/Spawning/BP_EnemySpawner.BP_EnemySpawner_C"))
  (set `self.spawners` _outactors))

(fn `NewWave`
  (`/Engine/EditorBlueprintResources/StandardMacros.IncrementInt` (`self.WaveNumber`)
    (:`  `
      (`self.GetSpawners`)
      (`self.StartWave`))))

(fn `OnEnemyDefeated`
  (bind _result (`/Engine/EditorBlueprintResources/StandardMacros.DecrementInt` (`self.EnemyRemaining`))
    (:`  `
      (if (< _result (`self.EnemyMaxCount`))
        (if (<= (`self.EnemyRemaining`) 0)
          (`self.EnterTransition` 5.0))
        (else
          (bind _enem (`self.GetEnemyFromPool`))
          (`/Game/Enemies/Spawning/BP_EnemySpawner.AddEnemyToQueue` (`KismetArrayLibrary.Array_Random` (`self.spawners`)) _enem))))))

(fn `StartWave`
  (bind _outitem (`KismetArrayLibrary.Array_Random` (`self.spawners`)))
  (`self.BuildEnemyPool`)
  (for _ (range (`KismetMathLibrary.Min` (`self.GetPoolSize`) (`self.EnemyMaxCount`)))
    (bind _enem (`self.GetEnemyFromPool` :!label _label))
    (if (`KismetSystemLibrary.IsValid` _outitem)
      (`/Game/Enemies/Spawning/BP_EnemySpawner.AddEnemyToQueue` _outitem _enem)
      (else
        (goto _label)))))

(fn `UserConstructionScript`)